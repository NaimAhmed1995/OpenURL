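; BP_OpenURL is a Pixel Streaming actor that sends browser commands from the game on key presses.
; On BeginPlay it enables input, shows the WBP_OpenURL widget and disables the player character's movement.
; E sends a launchUrl command with the URL, and R sends a browser-side mouse cursor change.
; SendResponse joins the JSON string pieces and passes them to the PixelStreamingInput component on the player controller.
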(event `self.ReceiveBeginPlay`
  (bind _returnvalue (`GameplayStatics.GetPlayerController` 0))
  ;[0 0 0] Enable input and Disable player movement
  (`/Engine/EditorBlueprintResources/StandardMacros.IsValid` _returnvalue
    (:`Is Valid`
      (`self.EnableInput` _returnvalue)
      (bind _returnvalue_2 (`|GenericCreateObject` "/E3DSFeatures/UI/WBP_OpenURL.WBP_OpenURL_C"))
      (`UserWidget.AddToViewport` _returnvalue_2 0)
      (`CharacterMovementComponent.DisableMovement` (`Character.CharacterMovement` (`GameplayStatics.GetPlayerCharacter` 0))))))

(event `Key|E`
  (params (Key :type "Key Structure"))
  ;[0 0 0] Press E for Open URL in New Tab
  (:`Pressed`
    (`self.Send Response` "{\"cmd\":\"launchUrl\",\"value\":\"" (`self.URL`) "\"}")))

(event `Key|R`
  (params (Key :type "Key Structure"))
  (:`Pressed`
    (`self.Send Response` "{\"cmd\":\"setBrowserSideMouseCursorTo\",\"value\":\" " (`self.MouseCourserChangeCommand`) "\"}")))

(fn `Send Response`
  (params (CMD :type String) (Value :type String) (Last :type String))
  (bind _returnvalue (`self.GetComponentByClass` (`GameplayStatics.GetPlayerController` 0) (`self.Set Pixel streaming Input`)))
  (`/Engine/EditorBlueprintResources/StandardMacros.IsValid` (`GameplayStatics.GetPlayerCharacter` 0)
    (:`Is Valid`
      (`/Engine/EditorBlueprintResources/StandardMacros.IsValid` _returnvalue
        (:`Is Valid`
          (`PixelStreamingInput.SendPixelStreamingResponse` _returnvalue (`KismetStringLibrary.Concat_StrStr` (`KismetStringLibrary.Concat_StrStr` (`KismetSystemLibrary.MakeLiteralString` CMD) (`KismetSystemLibrary.MakeLiteralString` Value)) (`KismetSystemLibrary.MakeLiteralString` Last))))))))

(fn `UserConstructionScript`)